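; BP_DronePawn is a player-controlled drone pawn driven by Enhanced Input.
; On BeginPlay it adds the IMC_Drone mapping context, shows the mouse cursor and sets Game and UI input mode.
; IA_Move feeds its X and Y axes into movement input along the actor's right and forward vectors.
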(event `self.ReceiveBeginPlay`
  (bind _asplayer_controller (cast `PlayerController` (`self.GetController`)))
  (`EnhancedInputSubsystemInterface.AddMappingContext` (pcsubsystem `EnhancedInputLocalPlayerSubsystem` _asplayer_controller) "/Game/main_character/IMC_Drone.IMC_Drone" 0 (struct))
  (set `PlayerController.bShowMouseCursor` true _asplayer_controller)
  (`WidgetBlueprintLibrary.SetInputMode_GameAndUIEx` _asplayer_controller null))

(event `EnhancedInput|/Game/main_character/IA_Move`
  (params (ActionValue :type "Vector2D Structure") (ElapsedSeconds :type "Float (double-precision)") (TriggeredSeconds :type "Float (double-precision)") (InputAction :type "InputAction Object Reference" :default "/Game/main_character/IA_Move.IA_Move"))
  (bind (_x _y) (`KismetMathLibrary.BreakVector2D` ActionValue))
  (:`Triggered`
    (`self.AddMovementInput` (`self.GetActorRightVector`) _x)
    (`self.AddMovementInput` (`self.GetActorForwardVector`) _y)))

(fn `UserConstructionScript`)